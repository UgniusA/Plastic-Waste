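; Melee enemy character that patrols three points until it sees the third-person player, then chases to attacking range.
; Tick checks line of sight, yaws toward the player and picks patrol or chase via AIMoveTo.
; FindPlayer re-runs itself on a short delay, updating attack state, while completed moves adjust walk speed as stamina loss.
; Animation events for attacking, which damages player Health, and random blocking are defined but not called here.
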(event Custom|Search%20Animation
  ;[1 1 1] Animation All V2
  (Components|Animation|PlayAnimation (Variables|Default|GetMixamo_Base) "/Game/ThirdPersonCPP/Animations/Mixamo_Base_Anim_mixamo_com.Mixamo_Base_Anim_mixamo_com" true))

(event Custom|Attack%20Animation
  (bind _mixamo_base (Variables|Default|GetMixamo_Base))
  ;[1 1 1] Animation All V2
  (Components|Animation|PlayAnimation _mixamo_base "/Game/ThirdPersonCPP/Animations/Sword_And_Shield_Slash_mixamo_com.Sword_And_Shield_Slash_mixamo_com" false)
  (CallFunction|DamagePlayer)
  (Components|Animation|PlayAnimation _mixamo_base "/Game/ThirdPersonCPP/Animations/Sword_And_Shield_Slash__1__mixamo_com.Sword_And_Shield_Slash__1__mixamo_com" false)
  (CallFunction|DamagePlayer)
  (Components|Animation|PlayAnimation _mixamo_base "/Game/ThirdPersonCPP/Animations/Sword_And_Shield_Kick_mixamo_com.Sword_And_Shield_Kick_mixamo_com" false)
  (CallFunction|DamagePlayer))

(event Custom|Find%20Player
  (bind _self self)
  ;[1 1 1] Find Player
  (if (and (Variables|Default|Getis%20In%20LOS) (>= (Transformation|GetDistanceTo (Variables|Default|GetPlayer)) (Variables|Default|GetMinimum%20Attacking%20Distance)))
    (AI|AIMoveTo _self "0, 0,0.000000" (Variables|Default|GetPlayer) 5.0 false
      (:then
        (Variables|Default|Setis%20Searching true)
        (Utilities|FlowControl|Delay 0.2 :!label _label)
        (CallFunction|FindPlayer)
        (CallFunction|Attacking))
      (:OnSuccess
        (CallFunction|StaminaLoss :!label _label_2)))
    (else
      (AI|AIMoveTo _self "0,0.000000, 0" _self 5.0 false
        (:then
          (Variables|Default|Setis%20Searching false)
          (goto _label))
        (:OnSuccess
          (goto _label_2))))))

(event Custom|Stamina%20Loss
  (bind _default_speed (Variables|Default|GetDefault%20Speed))
  (bind _charactermovement (Variables|Character|GetCharacterMovement))
  ;[1 1 1] Stamina Loss Over Time
  (if (and (== (Variables|/Script/Engine.CharacterMovementComponent|GetMaxWalkSpeed (Variables|Character|GetCharacterMovement)) 6e+02) (Variables|Default|Getis%20In%20LOS))
    (Utilities|FlowControl|Delay 2.0)
    (Variables|/Script/Engine.CharacterMovementComponent|SetMaxWalkSpeed _charactermovement (/ _default_speed 2.0))
    (else
      (Variables|/Script/Engine.CharacterMovementComponent|SetMaxWalkSpeed _charactermovement _default_speed))))

(event Custom|Patrol%20or%20Search
  ;[1 1 1] Patrol or Search
  (if (not (Variables|Default|Getis%20In%20LOS))
    (CallFunction|Patrol)
    (else
      (CallFunction|FindPlayer))))

(event Custom|Set%20Variables
  ;[1 1 1] Declare Variables
  (Variables|Default|SetDefault%20Speed 6e+02)
  (Variables|Default|SetMinimum%20Attacking%20Distance 1.5e+02))

(event Custom|Attacking
  ;[1 1 1] Attacking Bool
  (if (and (Variables|Default|Getis%20In%20LOS) (<= (Transformation|GetDistanceTo (Variables|Default|GetPlayer)) (Variables|Default|GetMinimum%20Attacking%20Distance)))
    (Variables|Default|Setis%20Attacking true)
    (else
      (Variables|Default|Setis%20Attacking false))))

(event Custom|Block%20Animation
  ;[1 1 1] Animation All V2
  (Components|Animation|PlayAnimation (Variables|Default|GetMixamo_Base) "/Game/ThirdPersonCPP/Animations/Sword_And_Shield_Impact_mixamo_com.Sword_And_Shield_Impact_mixamo_com" false))

(event Custom|Idle%20Animation
  ;[1 1 1] Animation All V2
  (Components|Animation|PlayAnimation (Variables|Default|GetMixamo_Base) "/Game/ThirdPersonCPP/Animations/Idle_mixamo_com.Idle_mixamo_com" true))

(event Custom|Damage%20Player
  ;[1 1 1] Damage Player
  (bind _returnvalue (Actor|GetActorOfClass "/Game/ThirdPersonCPP/Blueprints/ThirdPersonCharacter.ThirdPersonCharacter_C"))
  (Variables|/Game/ThirdPersonCPP/Blueprints/ThirdPersonCharacter.ThirdPersonCharacter_C|SetHealth _returnvalue (- (Variables|/Game/ThirdPersonCPP/Blueprints/ThirdPersonCharacter.ThirdPersonCharacter_C|GetHealth _returnvalue) (Variables|Default|GetDamage%20Amount))))

(event Custom|Block%20Chance
  ;[1 1 1] Blocking
  (if (Math|Random|RandomBoolwithWeight (Variables|Default|GetChance%20to%20Block))
    (CallFunction|BlockAnimation)
    (else
      (CallFunction|IdleAnimation))))

(event Custom|Check%20Sight%20Line
  ;[1 1 1] Check Line of Sight to Player
  (if (Controller|LineOfSightTo (Pawn|GetController) (Variables|Default|GetPlayer) "0, 0, 0" false)
    (Variables|Default|Setis%20In%20LOS true)
    (else
      (Variables|Default|Setis%20In%20LOS false))))

(event Custom|Patrol
  (bind _self self)
  ;[1 1 1] Patrol
  (AI|AIMoveTo _self "0, 0, 0" (Variables|Default|GetPatrol%20Location%201) 5.0 false
    (:OnSuccess
      (Utilities|FlowControl|Delay 3.0)
      (AI|AIMoveTo _self "0, 0, 0" (Variables|Default|GetPatrol%20Location%202) 5.0 false
        (:OnSuccess
          (Utilities|FlowControl|Delay 3.0)
          (AI|AIMoveTo _self "0, 0, 0" (Variables|Default|GetPatrol%20Location%203) 5.0 false))))))

(event Custom|Look%20At%20Player
  (params (DeltaSeconds :type Float%20%28single-precision%29))
  ;[1 1 1] Look at Player
  (if (or (Variables|Default|Getis%20Searching) (Variables|Default|Getis%20Attacking))
    (Transformation|SetActorRotation (Math|Rotator|MakeRotator 0.0 0.0 (.yaw (Math|Rotator|FindLookatRotation (Transformation|GetWorldLocation (Variables|Collision|GetCapsuleComponent)) (Transformation|GetActorLocation (Variables|Default|GetPlayer))))))
    (else
      (Transformation|SetActorRotation (Math|Rotator|MakeRotator 0.0 0.0 0.0)))))

(event EventTick
  (params (DeltaSeconds :type Float%20%28single-precision%29))
  ;[1 1 1] Update
  (CallFunction|CheckSightLine)
  (CallFunction|LookatPlayer 0.0)
  (CallFunction|PatrolorSearch))

(event EventBeginPlay
  ;[1 1 1] Find Player
  (bind _returnvalue (Actor|GetActorOfClass "/Game/ThirdPersonCPP/Blueprints/ThirdPersonCharacter.ThirdPersonCharacter_C"))
  (Variables|Default|SetPlayer _returnvalue)
  (CallFunction|SetVariables))

(fn ConstructionScript)