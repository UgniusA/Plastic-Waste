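; ExplodingEnemyV2 is an enemy that chases the ThirdPersonCharacter and explodes when its capsule hits something.
; On BeginPlay it finds and caches the player, then a recursive MoveToPlayer event reissues AIMoveTo on a short delay while the player is beyond a minimum distance.
; Inside that distance it clears IsWithinRange and targets itself instead.
; Any capsule hit activates the particle system and destroys the actor after a brief delay.
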(event OnComponentHit(CapsuleComponent)
  (params (HitComponent :type Primitive%20Component%20Object%20Reference) (OtherActor :type Actor%20Object%20Reference) (OtherComp :type Primitive%20Component%20Object%20Reference) (NormalImpulse :type Vector :default "0, 0, 0") (Hit :type Hit%20Result%20Structure%20%28by%20ref%29))
  ;[1 1 1] Explosion
  (Components|Activation|Activate (Variables|Default|GetParticleSystem) false)
  (Utilities|FlowControl|Delay 0.3)
  (Actor|DestroyActor))

(event Custom|Move%20To%20Player
  ;[1 1 1] Find Player
  (if (>= (Transformation|GetDistanceTo (Variables|Default|GetPlayer)) 1e+02)
    (Variables|Default|Setis%20Within%20Range true)
    (AI|AIMoveTo self "0, 0, 0" (Variables|Default|GetPlayer) 5.0 false
      (:then
        _))
    (else
      (Variables|Default|Setis%20Within%20Range false)
      (AI|AIMoveTo 0 "0, 0, 0" self 5.0 false
        (:then
          _))))
  (Utilities|FlowControl|Delay 0.2)
  (CallFunction|MovetoPlayer))

(event EventBeginPlay
  ;[1 1 1] Find Player
  (bind _returnvalue (Actor|GetActorOfClass "/Game/ThirdPersonCPP/Blueprints/ThirdPersonCharacter.ThirdPersonCharacter_C"))
  (bind _output_get (Variables|Default|SetPlayer _returnvalue))
  (Development|PrintString (Utilities|GetDisplayName _output_get))
  (CallFunction|MovetoPlayer))

(fn ConstructionScript)