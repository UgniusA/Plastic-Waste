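; An actor that can smoothly turn to face the player's ThirdPersonCharacter while its FacePlayer flag is set.
; BeginPlay finds and caches the character with GetActorOfClass and prints its display name.
; Each Tick interpolates the whole actor's rotation toward the look-at rotation with RInterpTo at a fixed speed.
; A local-rotation node and its RotationSpeed input are leftovers that never run.
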(event EventBeginPlay
  (bind _returnvalue (Actor|GetActorOfClass "/Game/ThirdPersonCPP/Blueprints/ThirdPersonCharacter.ThirdPersonCharacter_C"))
  (bind _output_get (Variables|Default|SetPlayer _returnvalue))
  (Development|PrintString (Utilities|GetDisplayName _output_get)))

(event EventTick
  (params (DeltaSeconds :type Float%20%28single-precision%29))
  ;[1 1 1] V1
  (Variables|Default|SetDelta DeltaSeconds)
  (if (Variables|Default|GetFace%20Player)
    (Transformation|SetActorRotation (Math|Interpolation|RInterpTo (Transformation|GetActorRotation) (Math|Rotator|FindLookatRotation (Transformation|GetActorLocation) (Transformation|GetActorLocation (Variables|Default|GetPlayer))) (Variables|Default|GetDelta) 2.0))))

(fn ConstructionScript)