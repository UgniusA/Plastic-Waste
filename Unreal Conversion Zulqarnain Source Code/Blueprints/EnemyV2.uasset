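; EnemyV2 is an enemy pawn that turns to face the ThirdPersonCharacter every tick and has an unfinished patrol-or-chase behavior.
; BeginPlay finds the player and clears IsAlerted, so it takes the Patrol branch, whose AIMoveTo has no inputs.
; The chase branch re-runs AI MoveTo on a short delay, toggling IsWalking by distance.
; CheckBool is empty, and the patrol-point loop is disconnected.
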(event Custom|Move%20To%20Player
  ;[1 1 1] Searching
  (if (>= (Transformation|GetDistanceTo (Variables|Default|GetPlayer)) 1e+02)
    (Variables|Default|Setis%20Walking true)
    (AI|AIMoveTo self "0, 0, 0" (Variables|Default|GetPlayer) 5.0 false
      (:then
        _))
    (else
      (Variables|Default|Setis%20Walking false)
      (AI|AIMoveTo 0 "0, 0, 0" self 5.0 false
        (:then
          _))))
  (Utilities|FlowControl|Delay 0.2)
  (CallFunction|MovetoPlayer)
  (CallFunction|CheckBool))

(event Custom|Patrol%20or%20Search
  ;[1 1 1] Patroling or Searching
  (if (Variables|Default|Getis%20Alerted)
    (CallFunction|MovetoPlayer)
    (else
      (CallFunction|Patrol))))

(event Custom|Patrol
  (AI|AIMoveTo 0 "0, 0, 0" 0 5.0 false))

(event Custom|Check%20Bool)

(event EventBeginPlay
  ;[1 1 1] Find Player
  (Variables|Default|Setis%20Alerted false)
  (bind _returnvalue (Actor|GetActorOfClass "/Game/ThirdPersonCPP/Blueprints/ThirdPersonCharacter.ThirdPersonCharacter_C"))
  (bind _output_get (Variables|Default|SetPlayer _returnvalue))
  (Development|PrintString (Utilities|GetDisplayName _output_get))
  (CallFunction|PatrolorSearch))

(event EventTick
  (params (DeltaSeconds :type Float%20%28single-precision%29))
  ;[1 1 1] Look at Player
  (Transformation|SetActorRotation (Math|Rotator|MakeRotator 0.0 0.0 (.yaw (Math|Rotator|FindLookatRotation (Transformation|GetWorldLocation (Variables|Collision|GetCapsuleComponent)) (Transformation|GetActorLocation (Variables|Default|GetPlayer)))))))

(fn ConstructionScript)