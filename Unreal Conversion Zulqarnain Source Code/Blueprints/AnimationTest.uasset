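; Test actor for playing sword-and-shield animations on a Mixamo skeletal mesh from number keys.
; Keys 1-3 set walk, attack and randomized block flags; key 2 also starts a DoOnce-gated attack chain that key 4 re-arms.
; The chain sequences clips by polling IsPlaying with Delay loops, then starts a looping animation.
; SelectAnimation maps the flags to clips, but its only call here is disconnected, so walk and block trigger no animation themselves.
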(event Custom|Select%20Animation
  (bind _mixamo_base (Variables|Default|GetMixamo_Base))
  (if (Variables|Default|Getis%20Walking)
    (Components|Animation|PlayAnimation _mixamo_base "/Game/ThirdPersonCPP/Animations/Sword_And_Shield_Walk_mixamo_com.Sword_And_Shield_Walk_mixamo_com" true)
    (elif (Variables|Default|GetIs%20Attacking)
      (Components|Animation|PlayAnimation _mixamo_base 0 false)
      (if (Audio|Components|Audio|IsPlaying _mixamo_base) :!label _label
        (Utilities|FlowControl|Delay 0.5)
        (goto _label)
        (else
          (Components|Animation|PlayAnimation _mixamo_base 0 false)
          (if (Audio|Components|Audio|IsPlaying _mixamo_base) :!label _label_2
            (Utilities|FlowControl|Delay 0.5)
            (goto _label_2)
            (else
              (Components|Animation|PlayAnimation _mixamo_base 0 false)
              (Utilities|FlowControl|Delay 0.5)
              (Variables|Default|SetIs%20Attacking false)))))
      (elif (Variables|Default|Getis%20Blocking)
        (Components|Animation|PlayAnimation _mixamo_base 0 false)
        (Utilities|FlowControl|Delay 0.2)
        (Variables|Default|Setis%20Blocking false)
        (else
          (Components|Animation|PlayAnimation _mixamo_base 0 true))))))

(event EventBeginPlay
  (Input|EnableInput (Game|GetPlayerController 0))
  (Variables|Default|SetIs%20Attacking true))

(event Collision|EventActorBeginOverlap
  (params (OtherActor :type Actor%20Object%20Reference)))

(event EventTick
  (params (DeltaSeconds :type Float%20%28single-precision%29)))

(event Input|KeyboardEvents|2
  (params (Key :type Key%20Structure :default "None"))
  (:Pressed
    (Variables|Default|SetIs%20Attacking true)))

(event Input|KeyboardEvents|1
  (params (Key :type Key%20Structure :default "None"))
  (:Pressed
    (Variables|Default|Setis%20Walking true))
  (:Released
    (Variables|Default|Setis%20Walking false)))

(event Input|KeyboardEvents|3
  (params (Key :type Key%20Structure :default "None"))
  (:Released
    (if (Math|Random|RandomBoolwithWeight 0.4)
      (Variables|Default|Setis%20Blocking true)
      (else
        (Variables|Default|Setis%20Blocking false)))))

(event Input|KeyboardEvents|4
  (params (Key :type Key%20Structure :default "None"))
  (bind _mixamo_base (Variables|Default|GetMixamo_Base))
  (:Pressed
    (Development|PrintString "reset")
    (Utilities|FlowControl|DoOnce false) ; enters at Reset
  ))

(event Input|KeyboardEvents|2
  (params (Key :type Key%20Structure :default "None"))
  (bind _mixamo_base (Variables|Default|GetMixamo_Base))
  (:Pressed
    (Utilities|FlowControl|DoOnce false
      (:Completed
        (if (Variables|Default|GetIs%20Attacking)
          (Components|Animation|PlayAnimation _mixamo_base 0 false)
          (if (Audio|Components|Audio|IsPlaying _mixamo_base) :!label _label
            (Utilities|FlowControl|Delay 0.5)
            (goto _label)
            (else
              (Components|Animation|PlayAnimation _mixamo_base 0 false)
              (if (Audio|Components|Audio|IsPlaying _mixamo_base) :!label _label_2
                (Utilities|FlowControl|Delay 0.5)
                (goto _label_2)
                (else
                  (Components|Animation|PlayAnimation _mixamo_base 0 false)
                  (if (Audio|Components|Audio|IsPlaying _mixamo_base) :!label _label_3
                    (Utilities|FlowControl|Delay 0.5)
                    (goto _label_3)
                    (else
                      (Components|Animation|PlayAnimation _mixamo_base 0 true)
                      (Utilities|FlowControl|Delay 0.2)
                      (Variables|Default|SetIs%20Attacking false)))))))
          (else
            (Development|PrintString "Hello")))))))

(fn ConstructionScript)