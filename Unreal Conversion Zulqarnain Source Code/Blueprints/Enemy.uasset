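; Enemy actor that constantly turns to face the player character and chases it using AI movement.
; Tick smoothly interpolates rotation toward the player, cached on BeginPlay.
; MoveToPlayer re-runs itself after a short delay, setting IsWalking by a distance threshold and requesting a move toward the player when not yet close.
; CheckBool only prints the walking or found state; animation nodes are left unconnected.
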(event Custom|Move%20To%20Player
  ;[1 1 1] Move To Player
  (if (>= (Transformation|GetDistanceTo (Variables|Default|GetAs%20Third%20Person%20Character)) 1e+02)
    (Variables|Default|Setis%20Walking true)
    (AI|AIMoveTo self "0, 0, 0" (Variables|Default|GetAs%20Third%20Person%20Character) 5.0 false
      (:then
        _))
    (else
      (Variables|Default|Setis%20Walking false)
      (AI|AIMoveTo 0 "0, 0, 0" self 5.0 false
        (:then
          _))))
  (Utilities|FlowControl|Delay 0.2)
  (CallFunction|MovetoPlayer)
  (CallFunction|CheckBool))

(event Custom|Play%20Walking%20Anim
  ;[1 1 1] Is Walking Bool
)

(event Custom|Check%20Bool
  ;[1 1 1] Is Walking Bool
  (if (Variables|Default|Getis%20Walking)
    (Development|PrintString "Walking")
    (else
      (Development|PrintString "Found"))))

(event EventBeginPlay
  ;[1 1 1] Move To Player
  (bind _asthird_person_character (Utilities|Casting|CastToThirdPersonCharacter (Game|GetPlayerCharacter 0)))
  (Variables|Default|SetAs%20Third%20Person%20Character _asthird_person_character)
  (CallFunction|MovetoPlayer))

(event EventTick
  (params (DeltaSeconds :type Float%20%28single-precision%29))
  (Transformation|SetActorRotation (Math|Interpolation|RInterpTo (Transformation|GetActorRotation) (Math|Rotator|FindLookatRotation (Transformation|GetActorLocation) (Transformation|GetActorLocation (Variables|Default|GetAs%20Third%20Person%20Character))) 0.0 2e+01)))

(fn ConstructionScript)